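; BP_ReferenceManager sets up local multiplayer when play begins, despite its reference-manager name.
; It makes four successive CreatePlayer calls with automatic controller IDs, casts each new player's character to MannequinCharacterV2 and stores that controller ID in its PlayerControllerIndex.
; The steps are nested, so a failed cast or invalid character stops creation of the remaining players.
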(event EventBeginPlay
  (bind _returnvalue (Class|GameplayStatics|CreatePlayer -1))
  (bind _asmannequin_character_v2 (Utilities|Casting|CastToMannequinCharacterV2 (Game|GetPlayerCharacter (Class|GameplayStatics|GetPlayerControllerID _returnvalue))))
  (Utilities|IsValid _asmannequin_character_v2
    (:Is%20Valid
      (Variables|/Game/AdvancedLocomotion/Blueprints/Player_BP.Player_BP_C|SetPlayerControllerIndex _asmannequin_character_v2 (Class|GameplayStatics|GetPlayerControllerID _returnvalue))
      (bind _returnvalue_2 (Class|GameplayStatics|CreatePlayer -1))
      (bind _asmannequin_character_v2_2 (Utilities|Casting|CastToMannequinCharacterV2 (Game|GetPlayerCharacter (Class|GameplayStatics|GetPlayerControllerID _returnvalue_2))))
      (Utilities|IsValid _asmannequin_character_v2_2
        (:Is%20Valid
          (Variables|/Game/AdvancedLocomotion/Blueprints/Player_BP.Player_BP_C|SetPlayerControllerIndex _asmannequin_character_v2_2 (Class|GameplayStatics|GetPlayerControllerID _returnvalue_2))
          (bind _returnvalue_3 (Class|GameplayStatics|CreatePlayer -1))
          (bind _asmannequin_character_v2_3 (Utilities|Casting|CastToMannequinCharacterV2 (Game|GetPlayerCharacter (Class|GameplayStatics|GetPlayerControllerID _returnvalue_3))))
          (Utilities|IsValid _asmannequin_character_v2_3
            (:Is%20Valid
              (Variables|/Game/AdvancedLocomotion/Blueprints/Player_BP.Player_BP_C|SetPlayerControllerIndex _asmannequin_character_v2_3 (Class|GameplayStatics|GetPlayerControllerID _returnvalue_3))
              (bind _returnvalue_4 (Class|GameplayStatics|CreatePlayer -1))
              (bind _asmannequin_character_v2_4 (Utilities|Casting|CastToMannequinCharacterV2 (Game|GetPlayerCharacter (Class|GameplayStatics|GetPlayerControllerID _returnvalue_4))))
              (Utilities|IsValid _asmannequin_character_v2_4
                (:Is%20Valid
                  (Variables|/Game/AdvancedLocomotion/Blueprints/Player_BP.Player_BP_C|SetPlayerControllerIndex _asmannequin_character_v2_4 (Class|GameplayStatics|GetPlayerControllerID _returnvalue_4)))))))))))

(event Collision|EventActorBeginOverlap
  (params (OtherActor :type Actor%20Object%20Reference)))

(event EventTick
  (params (DeltaSeconds :type Float%20%28single-precision%29)))

(fn ConstructionScript)