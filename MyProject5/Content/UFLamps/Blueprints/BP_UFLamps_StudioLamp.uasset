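; BP_UFLamps_StudioLamp is a placeable studio lamp with an adjustable head and a switchable spot light.
; Its construction script pitches the Scene pivot component by RotateHead to tilt the head.
; When switched on, it applies bulb color and emissive strength to the head materials and sets the spot light color.
; When switched off, it hides the spot light and zeroes the emissive strength.
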(fn ConstructionScript
  ;[1 1 1] Initiate construction script, adjust rotation of the lamp head along its local Y axis
  ;;[1 1 1] Rotate Head static mesh component along the Y axis using the Scene component as pivot
  (Transformation|AddLocalRotation (Variables|Default|GetScene) (Math|Rotator|MakeRotator 0.0 (Variables|Default|GetRotate%20head) 0.0) false false)
  ;[1 1 1] Initiate construction script, check if Light is turned On/Off. By default the light source is enabled and the emissive is set to 3.0
  (if (Variables|Default|GetSwitch%20Light%20On/Off)
    ;[0 1 1] Light ON
    ;;[1 1 1] Get Bulb Color and set Emissive Color in the material of the static mesh component accordingly
    (Rendering|Material|SetVectorParameterValueonMaterials (Variables|Default|GetStudioLamp_Head) "Emissive Color" (Math|Conversions|ToVector(LinearColor) (Variables|Default|GetBulb%20Color)))
    ;;[1 1 1] Get Emissive Strength and set Emissive Strength in the material of the static mesh component accordingly
    (Rendering|Material|SetScalarParameterValueonMaterials (Variables|Default|GetStudioLamp_Head) "Emissive Strength" (Variables|Default|GetEmissive%20Strength))
    ;;[1 1 1] Get Light Color and set color of the light source component accordingly
    (Rendering|Components|Light|SetLightColor (Variables|Default|GetStudioLamp_SpotLight) (Variables|Default|GetLight%20Color) true)
    (else
      ;[1 0.1216 0] Light OFF
      ;;[1 1 1] Disable light source component
      (Rendering|SetVisibility (Variables|Default|GetStudioLamp_SpotLight) false false)
      ;;[1 1 1] Set Emissive Strength in the material of the static mesh component  to 0
      (Rendering|Material|SetScalarParameterValueonMaterials (Variables|Default|GetStudioLamp_Head) "Emissive Strength" 0.0))))