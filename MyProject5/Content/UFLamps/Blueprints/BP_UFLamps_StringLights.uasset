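; String lights prop that builds a cable with evenly spaced bulbs along an editable spline.
; The construction script adds a bulb mesh with slight random yaw and a point light below it at each distance step.
; User parameters set color, intensity, emissive and radius, with an on/off switch and optional weighted random unlit bulbs.
; Spline mesh segments between consecutive points form the cable; the event graph is unused.
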(event EventBeginPlay)

(event Collision|EventActorBeginOverlap
  (params (OtherActor :type Actor%20Object%20Reference)))

(event EventTick
  (params (DeltaSeconds :type Float%20%28single-precision%29)))

(fn ConstructionScript
  (bind _lights_distance (Variables|Default|GetLights%20Distance))
  ;[1 1 1] Initiate construction script, determine number of lights used to populate the Spline Component based Light Distance
  (for _index (range 0 (- (.ReturnValue (Math|Float|Division(WholeandRemainder) (Spline|GetSplineLength (Variables|Default|GetString)) (Variables|Default|GetLights%20Distance))) 1))
    ;[0 1 0.3718] Create static meshes & point light sources based on user input data
    (bind _returnvalue (AddComponent|AddStaticMeshComponent false (Math|Transform|MakeTransform (Spline|GetLocationatDistanceAlongSpline (Variables|Default|GetString) (+ (* _index _lights_distance) _lights_distance) "Local") (Math|Rotator|MakeRotator 0.0 0.0 (Math|Random|RandomFloatinRange -15.0 15.0))))) ; Spawn Bulb meshes along spline based on parameters set by user
    (bind _returnvalue_2 (AddComponent|AddPointLightComponent false (Math|Transform|MakeTransform (- (Spline|GetLocationatDistanceAlongSpline (Variables|Default|GetString) (+ (* _index _lights_distance) _lights_distance) "Local") "0, 0,10.000000")))) ; Spawn Point Light along spline where Bulb mesh has been created
    ;[1 1 1] Set Light Attenuation Radius
    (Rendering|Lighting|SetAttenuationRadius _returnvalue_2 (Variables|Default|GetLight%20Attenuation%20Radius))
    ;[1 1 1] Initiate construction script, check if Light is turned On/Off. By default the light source is enabled and the emissive is set to 3.0
    (if (Variables|Default|GetSwitch%20Light%20On/Off)
      ;[0.4067 0 1] Randomization branch
      ;;[1 1 1] Check if Randomize option is turned ON. If it is ON get the value of Randomization Effect
      (if (Variables|Default|GetRandomize)
        (if (Math|Random|RandomBoolwithWeight (Variables|Default|GetRandomization%20effect))
          ;;[1 0.1237 0] Light OFF
          ;;;[1 1 1] Disable light source component
          (Rendering|Components|Light|SetIntensity _returnvalue_2 0.0)
          ;;;[1 1 1] Set Emissive Strength in the material of the static mesh component  to 0
          (Rendering|Material|SetScalarParameterValueonMaterials _returnvalue "Emissive Strength" 0.0)
          (else
            ;;[0 0.9978 1] Light ON
            (Rendering|Components|Light|SetIntensity _returnvalue_2 (Variables|Default|GetLight%20Intensity))
            ;;;[1 1 1] Get Bulb Color and set Emissive Color in the material of the static mesh component accordingly
            (Rendering|Material|SetVectorParameterValueonMaterials _returnvalue "Emissive Color" (Math|Conversions|ToVector(LinearColor) (Variables|Default|GetEmissive%20Color)))
            ;;;[1 1 1] Get Emissive Strength and set Emissive Strength in the material of the static mesh component accordingly
            (Rendering|Material|SetScalarParameterValueonMaterials _returnvalue "Emissive Strength" (Variables|Default|GetEmissive%20Strength))
            ;;;[1 1 1] Get Light Color and set color of the light source component accordingly
            (Rendering|Components|Light|SetLightColor _returnvalue_2 (Variables|Default|GetLight%20Color) true)))
        (else
          ;[1 1 1] Default On/Off branch
          ;;[0 0.9978 1] Light ON
          (Rendering|Components|Light|SetIntensity _returnvalue_2 (Variables|Default|GetLight%20Intensity))
          ;;;[1 1 1] Get Bulb Color and set Emissive Color in the material of the static mesh component accordingly
          (Rendering|Material|SetVectorParameterValueonMaterials _returnvalue "Emissive Color" (Math|Conversions|ToVector(LinearColor) (Variables|Default|GetEmissive%20Color)))
          ;;;[1 1 1] Get Emissive Strength and set Emissive Strength in the material of the static mesh component accordingly
          (Rendering|Material|SetScalarParameterValueonMaterials _returnvalue "Emissive Strength" (Variables|Default|GetEmissive%20Strength))
          ;;;[1 1 1] Get Light Color and set color of the light source component accordingly
          (Rendering|Components|Light|SetLightColor _returnvalue_2 (Variables|Default|GetLight%20Color) true)))
      (else
        ;;[1 0.1237 0] Light OFF
        ;;;[1 1 1] Disable light source component
        (Rendering|Components|Light|SetIntensity _returnvalue_2 0.0)
        ;;;[1 1 1] Set Emissive Strength in the material of the static mesh component  to 0
        (Rendering|Material|SetScalarParameterValueonMaterials _returnvalue "Emissive Strength" 0.0))))
  ;[1 0.8679 0.2464] Attach Cable static mesh to Spline Component. If a new control point is added to the spline, attach a new Cable mesh to the previous one
  (for _index_2 (range 0 (- (Spline|GetNumberOfSplinePoints (Variables|Default|GetString)) 2))
    (bind _returnvalue_3 (AddComponent|AddSplineMeshComponent true))
    (Transformation|AttachComponentToComponent _returnvalue_3 (Variables|Default|GetDefaultSceneRoot) "None" "KeepRelative" "KeepRelative" "KeepRelative" true)
    (SplineMesh|SetStartandEnd _returnvalue_3 (.Location (Spline|GetLocationandTangentatSplinePoint (Variables|Default|GetString) _index_2 "Local")) (.Tangent (Spline|GetLocationandTangentatSplinePoint (Variables|Default|GetString) _index_2 "Local")) (.Location (Spline|GetLocationandTangentatSplinePoint (Variables|Default|GetString) (+ _index_2 1) "Local")) (.Tangent (Spline|GetLocationandTangentatSplinePoint (Variables|Default|GetString) (+ _index_2 1) "Local")) true :!class /Script/Engine.SplineMeshComponent)))