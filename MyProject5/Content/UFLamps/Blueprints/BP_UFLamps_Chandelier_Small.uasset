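; Small chandelier lamp actor, configured entirely in its Construction Script with no active runtime logic.
; A loop adds chain segment meshes at 7-unit vertical steps to build the hanging chain from NumberOfChainSegments.
; SwitchLightOnOff then either applies bulb emissive color and strength to the mesh materials and sets the point light color, or hides the light and zeroes the emissive.
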(event EventBeginPlay)

(event Collision|EventActorBeginOverlap
  (params (OtherActor :type Actor%20Object%20Reference)))

(event EventTick
  (params (DeltaSeconds :type Float%20%28single-precision%29)))

(fn ConstructionScript
  ;[1 1 1] Initiate construction script, get the number of chain segments making up the chain that is holding the chandelier hanging from the ceiling and run them through a loop. When the loop is finished adding the chain segments on top of one another, continue to check if the lamp is turned ON
  (for _index (range 0 (- (Variables|Default|GetNumberOfChainSegments) 1)) ; ForLoop adding each chain segment on top of each other
    ;;[1 1 1] Attach the chain segments together to get one continuous body of chain holding the lamp hanging from the ceiling
    (AddComponent|AddStaticMeshComponent false (Math|Transform|MakeTransform (* "0, 0,7.000000" _index))))
  ;[1 1 1] Check if Light is turned On/Off. By default the light source is enabled and the emissive is set to 3.0
  (if (Variables|Default|GetSwitch%20Light%20On/Off)
    ;[0 1 1] Light ON
    ;;[1 1 1] Get Bulb Color and set Emissive Color in the material of the static mesh component accordingly
    (Rendering|Material|SetVectorParameterValueonMaterials (Variables|Default|GetChandelier2_StaticMesh) "Emissive Color" (Math|Conversions|ToVector(LinearColor) (Variables|Default|GetBulb%20Color)))
    ;;[1 1 1] Get Emissive Strength and set Emissive Strength in the material of the static mesh component accordingly
    (Rendering|Material|SetScalarParameterValueonMaterials (Variables|Default|GetChandelier2_StaticMesh) "Emissive Strength" (Variables|Default|GetEmissive%20Strength))
    ;;[1 1 1] Get Light Color and set color of the light source component accordingly
    (Rendering|Components|Light|SetLightColor (Variables|Default|GetChandelier2_PointLight) (Variables|Default|GetLight%20Color) true)
    (else
      ;[1 0.1216 0] Light OFF
      ;;[1 1 1] Disable light source component
      (Rendering|SetVisibility (Variables|Default|GetChandelier2_PointLight) false false)
      ;;[1 1 1] Set Emissive Strength in the material of the static mesh component  to 0
      (Rendering|Material|SetScalarParameterValueonMaterials (Variables|Default|GetChandelier2_StaticMesh) "Emissive Strength" 0.0))))