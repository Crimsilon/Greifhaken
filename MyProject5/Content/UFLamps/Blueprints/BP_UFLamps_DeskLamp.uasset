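; Desk lamp Blueprint with a static mesh and spot light, configured in the construction script by an on/off switch.
; When on, it pushes bulb color and emissive strength into the mesh material and sets the spot light's color.
; When off, it hides the spot light and zeroes the material's emissive strength.
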(fn ConstructionScript
  ;[1 1 1] Initiate construction script, check if Light is turned On/Off. By default the light source is enabled and the emissive is set to 3.0
  (if (Variables|Default|GetSwitch%20Light%20On/Off)
    ;[0 0.9978 1] Light ON
    ;;[1 1 1] Get Bulb Color and set Emissive Color in the material of the static mesh component accordingly
    (Rendering|Material|SetVectorParameterValueonMaterials (Variables|Default|GetDeskLamp_StaticMesh) "Emissive Color" (Math|Conversions|ToVector(LinearColor) (Variables|Default|GetBulb%20Color)))
    ;;[1 1 1] Get Emissive Strength and set Emissive Strength in the material of the static mesh component accordingly
    (Rendering|Material|SetScalarParameterValueonMaterials (Variables|Default|GetDeskLamp_StaticMesh) "Emissive Strength" (Variables|Default|GetEmissive%20Strength))
    ;;[1 1 1] Get Light Color and set color of the light source component accordingly
    (Rendering|Components|Light|SetLightColor (Variables|Default|GetDeskLamp_SpotLight) (Variables|Default|GetLight%20Color) true)
    (else
      ;[1 0.1237 0] Light OFF
      ;;[1 1 1] Disable light source component
      (Rendering|SetVisibility (Variables|Default|GetDeskLamp_SpotLight) false false)
      ;;[1 1 1] Set Emissive Strength in the material of the static mesh component  to 0
      (Rendering|Material|SetScalarParameterValueonMaterials (Variables|Default|GetDeskLamp_StaticMesh) "Emissive Strength" 0.0))))